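; BP_FloatingText is a short-lived text actor, filed under player feedback, that displays a message in the world.
; On BeginPlay it applies its text and colour variables to a TextRender component.
; Each Tick moves the text along negative local Z and shrinks its world size at constant, frame-rate-independent rates.
; An accumulated timer destroys the actor once it reaches its Lifetime.
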(event `self.ReceiveBeginPlay`
  (bind _textrender (`self.TextRender`))
  (`TextRenderComponent.K2_SetText` _textrender (`self.TextToDisplay`))
  (`TextRenderComponent.SetTextRenderColor` _textrender (`self.Colour`)))

(event `self.ReceiveTick`
  (params (DeltaSeconds :type "Float (single-precision)"))
  (bind _textrender (`self.TextRender`))
  (bind _output_get (set `self.Timer` (+ DeltaSeconds (`self.Timer`))))
  (if (>= _output_get (`self.Lifetime`))
    (`self.K2_DestroyActor`)
    (else
      (`SceneComponent.K2_AddLocalOffset` _textrender (`KismetMathLibrary.MakeVector` 0.0 0.0 (* DeltaSeconds -50.0)) false false)
      (`TextRenderComponent.SetWorldSize` _textrender (+ (* DeltaSeconds -10.0) (`TextRenderComponent.WorldSize` _textrender))))))

(fn `UserConstructionScript`)