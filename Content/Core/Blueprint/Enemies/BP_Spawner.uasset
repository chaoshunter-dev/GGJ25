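; BP_Spawner is an enemy spawner that periodically spawns actors around its own location, driven by a configuration.
; SetupConfiguration starts a looping timer that calls Spawn at the configured rate while the enemy count is below the limit.
; Spawn adds a random location offset, then records each new enemy.
; SetActorsToSpawn rolls each class's chance, picks randomly among those passing, and recurses if none pass.
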(fn `SetActorsToSpawn`
  (params (Enemies :type "Map of /Game/Core/Blueprint/Enemies/BP_EnemyPArent Class Reference to Float (double-precision)"))
  (returns (ActorClass :type "/Game/Core/Blueprint/Enemies/BP_EnemyPArent Class Reference"))
  (locals (LocalClass :type "Array of /Game/Core/Blueprint/Enemies/BP_EnemyPArent Class Reference"))
  (bind _localclass (`local.LocalClass`))
  (`BlueprintMapLibrary.Map_Keys` Enemies)
  (for _array_element _
    (if (<= (`KismetMathLibrary.RandomFloatInRange` 0.0 1.0) (`BlueprintMapLibrary.Map_Find` Enemies _array_element))
      (`BlueprintMapLibrary.Map_Add` Enemies)))
  (if (`KismetArrayLibrary.Array_IsEmpty` _localclass)
    (bind _actorclass (`self.SetActorsToSpawn` Enemies))
    (return _actorclass)
    (else
      (return (`KismetArrayLibrary.Array_Random` _localclass)))))

(fn `SetupConfiguration`
  (`KismetSystemLibrary.K2_SetTimer` null "Spawn" (`.SpawnRate_12_467A643C4C517363CB2FE3A72B37DB10` (break `/Game/Core/Blueprint/Enemies/DataType/S_EnemyConfig` (`self.Configuration`))) true))

(fn `Spawn`
  (bind (_enemytype _actors _spawnrate _spawnlimit) (break `/Game/Core/Blueprint/Enemies/DataType/S_EnemyConfig` (`self.Configuration`)))
  (if (< (`self.CurrentEnemyCount`) _spawnlimit)
    (bind _actorclass (`self.SetActorsToSpawn` _actors))
    (bind _returnvalue (`|SpawnActorFromClass` _actorclass (`KismetMathLibrary.MakeTransform` (+ (`self.K2_GetActorLocation`) (`KismetArrayLibrary.Array_Random` (`self.SpawnLocations`)))) "Undefined" "MultiplyWithRoot" null null))
    (`/Engine/EditorBlueprintResources/StandardMacros.IncrementInt` (`self.CurrentEnemyCount`)
      (:`  `
        (`KismetArrayLibrary.Array_Add` (`self.Enemies`) _returnvalue)))))

(fn `UserConstructionScript`)