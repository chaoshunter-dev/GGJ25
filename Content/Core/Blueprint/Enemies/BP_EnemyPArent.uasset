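; Base enemy Blueprint, likely a parent class, that chases the player character and damages what it hits.
; BeginPlay caches the player, resets health and passes it to the BP_EnemyHealth widget.
; Tick issues AIMoveTo toward the player, looping after a short delay, while Hit applies attack damage.
; OnDamaged only checks for depleted health, then spawns an explosion emitter, decrements BP_Spawner's enemy count and destroys the actor.
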(event `self.ReceiveBeginPlay`
  (bind _asbp_bubble_character (cast `/Game/Core/Blueprint/Player/BP_BubbleCharacter` (`GameplayStatics.GetPlayerCharacter` 0)))
  (bind _output_get (set `self.Player` _asbp_bubble_character))
  (set `self.PlayerLocation` (`self.K2_GetActorLocation` _output_get))
  (set `self.EnemyHealth` (`self.EnemyMaxHealth`))
  (`self.NewFunction`))

(event `self.ReceiveTick`
  (params (DeltaSeconds :type "Float (single-precision)"))
  (`|ExecutionSequence`
    (:`then_0`
      (`|AIMoveTo` self (`self.PlayerLocation`) (`self.Player`) 0.2 :!label _label
        (:`then`
          (`KismetSystemLibrary.Delay` 0.3)
          (goto _label))))))

(event `self.ReceiveHit`
  (params (MyComp :type "PrimitiveComponent Object Reference") (Other :type "Actor Object Reference") (OtherComp :type "PrimitiveComponent Object Reference") (bSelfMoved :type Boolean) (HitLocation :type "Vector Structure") (HitNormal :type "Vector Structure") (NormalImpulse :type "Vector Structure") (Hit :type "HitResult Structure (by ref)"))
  (`KismetSystemLibrary.PrintString` "Hello")
  (`GameplayStatics.ApplyDamage` Other (`self.EnemyAttackValue`)))

(fn `NewFunction`
  (bind _asbp_enemy_health (cast `/Game/Core/Blueprint/BP_EnemyHealth` (`WidgetComponent.GetUserWidgetObject` (`self.Widget`))))
  (set `/Game/Core/Blueprint/BP_EnemyHealth.health` (`self.EnemyHealth`) _asbp_enemy_health)
  (return))

(fn `OnDamaged`
  (if (<= (`self.EnemyHealth`) 0.0)
    (`MovementComponent.StopMovementImmediately` (`self.CharacterMovement`))
    (`GameplayStatics.SpawnEmitterAtLocation` "/Game/StarterContent/Particles/P_Explosion.P_Explosion" (`SceneComponent.K2_GetComponentLocation` (`self.Mesh`)) (struct) (3.0 3.0 30.0) true "None" false)
    (bind _returnvalue (`GameplayStatics.GetActorOfClass` "/Game/Core/Blueprint/Enemies/BP_Spawner.BP_Spawner_C"))
    (`/Engine/EditorBlueprintResources/StandardMacros.DecrementInt` (`/Game/Core/Blueprint/Enemies/BP_Spawner.CurrentEnemyCount` _returnvalue)
      (:`  `
        (`self.K2_DestroyActor`)))
    (else
      (return))))

(fn `UserConstructionScript`)