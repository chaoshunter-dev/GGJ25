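; BP_LaserEmitter is the laser source for the mirror puzzle, drawing a beam with a Cable component.
; UpdateLaser, called on BeginPlay rather than on Tick, line-traces forward from the Arrow and moves the cable's end to the impact point in local space.
; If it hits a BP_SpinningMirror component tagged Mirror, it calls ReflectLaser on that mirror, using the second tag to indicate whether the Right side was struck.
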(event `self.ReceiveBeginPlay`
  (`self.Event UpdateLaser`))

(event `self.ReceiveTick`
  (params (DeltaSeconds :type "Float (single-precision)")))

(event `Event UpdateLaser`
  (bind _arrow (`self.Arrow`))
  (bind _returnvalue (`SceneComponent.K2_GetComponentLocation` _arrow))
  (bind _outhit (`KismetSystemLibrary.LineTraceSingle` _returnvalue (+ _returnvalue (* (`SceneComponent.GetForwardVector` _arrow) 1000.0)) "TraceTypeQuery1"))
  (bind (_bblockinghit _binitialoverlap _time _distance _location _impactpoint _normal _impactnormal _physmat _hitactor _hitcomponent) (`GameplayStatics.BreakHitResult` _outhit))
  ;[1 1 1 0.4] Move cable
  (set `CableComponent.EndLocation` (`KismetMathLibrary.InverseTransformLocation` (`SceneComponent.K2_GetComponentToWorld` (`self.Cable`)) _impactpoint) (`self.Cable`))
  (bind _asbp_spinning_mirror (cast `/Game/Core/Blueprint/Interactables/Mirror/BP_SpinningMirror` _hitactor))
  (bind _componenttags (`ActorComponent.ComponentTags` _hitcomponent))
  (if (== (`|GetArrayItem` _componenttags) "Mirror")
    (`/Game/Core/Blueprint/Interactables/Mirror/BP_SpinningMirror.Event ReflectLaser` _asbp_spinning_mirror (== (`|GetArrayItem` _componenttags 1) "Right"))))

(fn `UserConstructionScript`)