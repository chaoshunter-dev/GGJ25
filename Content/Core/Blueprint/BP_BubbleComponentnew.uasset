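; Actor component for BP_ThirdPersonCharacternew that fires BP_PRojectile when the IA_Shoot input starts, with a cooldown between shots.
; BeginPlay caches the owning character, whose location, forward vector and rotation place each projectile just ahead of it.
; Firing clears CanShoot, and a Tick-driven timer restores it once ShootDelayTime has elapsed.
; Debug prints report startup, a failed owner cast and shots blocked by the cooldown.
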(event `self.ReceiveBeginPlay`
  (`KismetSystemLibrary.PrintString` "Hello")
  (bind _asbp_third_person_characternew (cast `/Game/Core/Blueprint/BP_ThirdPersonCharacternew` (`self.GetOwner`))
    (:`then`
      (set `self.Owning Character` _asbp_third_person_characternew))
    (:`CastFailed`
      (`KismetSystemLibrary.PrintString` "cast failed"))))

(event `self.ReceiveTick`
  (params (DeltaSeconds :type "Float (single-precision)"))
  (`self.Shot Reset Timer` DeltaSeconds))

(event `EnhancedInput|/Game/Core/Input/Actions/IA_Shoot`
  (params (ActionValue :type Boolean) (ElapsedSeconds :type "Float (double-precision)") (TriggeredSeconds :type "Float (double-precision)") (InputAction :type "InputAction Object Reference" :default "/Game/Core/Input/Actions/IA_Shoot.IA_Shoot"))
  (:`Started`
    (if (`self.CanShoot`)
      (`|SpawnActorFromClass` "/Game/StarterContent/Blueprints/BP_PRojectile.BP_PRojectile_C" (`self.Get Projectile Spawn Transform`) "Undefined" "MultiplyWithRoot" null null)
      (set `self.CanShoot` false)
      (else
        (`KismetSystemLibrary.PrintString` "Shoot delayed!" true true (struct :`R` 1.0 :`G` 0.077193 :`A` 1.0))))))

(fn `Get Projectile Spawn Transform`
  (returns (ReturnValue :type "Transform Structure"))
  (bind _owning_character (`self.Owning Character`))
  (return (`KismetMathLibrary.MakeTransform` (+ (* (`Actor.GetActorForwardVector` _owning_character) 100) (`Actor.K2_GetActorLocation` _owning_character)) (`Actor.K2_GetActorRotation` _owning_character))))

(fn `Shot Reset Timer`
  (params (DeltaTime :type "Float (double-precision)"))
  (if (not (`self.CanShoot`))
    (bind _output_get (set `self.ShootDelayTimer` (+ DeltaTime (`self.ShootDelayTimer`))))
    (if (>= _output_get (`self.ShootDelayTime`))
      (set `self.CanShoot` true)
      (set `self.ShootDelayTimer` 0.0))))