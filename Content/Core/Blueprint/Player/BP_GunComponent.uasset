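; Gun component for BP_BubbleCharacter that fires BP_PRojectile actors when the shoot input starts.
; It switches on the owner's fire type: base shot, powerup-gated rear and spread shots, or rapid fire delegated to the character.
; Base shots spawn from the head socket; rear and spread shots use yaw offsets around the owner.
; Only base fire starts the Tick-driven cooldown, during which shooting triggers the character's reloading feedback.
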(event `self.ReceiveBeginPlay`
  (`KismetSystemLibrary.PrintString` "Hello")
  (bind _asbp_bubble_character (cast `/Game/Core/Blueprint/Player/BP_BubbleCharacter` (`self.GetOwner`))
    (:`then`
      (set `self.Owning Character` _asbp_bubble_character))
    (:`CastFailed`
      (`KismetSystemLibrary.PrintString` "cast failed"))))

(event `self.ReceiveTick`
  (params (DeltaSeconds :type "Float (single-precision)"))
  (`self.Shot Reset Timer` DeltaSeconds))

(event `EnhancedInput|/Game/Core/Input/Actions/IA_Shoot`
  (params (ActionValue :type Boolean) (ElapsedSeconds :type "Float (double-precision)") (TriggeredSeconds :type "Float (double-precision)") (InputAction :type "InputAction Object Reference" :default "/Game/Core/Input/Actions/IA_Shoot.IA_Shoot"))
  (bind _owning_character (`self.Owning Character`))
  (:`Started`
    (if (`self.CanShoot`)
      (switch `/Game/Core/Blueprint/Data/E_FireType` (`/Game/Core/Blueprint/Player/BP_BubbleCharacter.FireTypes` _owning_character)
        (:`NewEnumerator0`
          (`self.Base Fire`))
        (:`NewEnumerator1`
          (`self.Rear Fire`))
        (:`NewEnumerator2`
          (`self.Spread Fire 1`))
        (:`NewEnumerator3`
          (`self.Spread Fire 2`))
        (:`NewEnumerator4`
          (`/Game/Core/Blueprint/Player/BP_BubbleCharacter.Powerup_RapidFire` _owning_character)))
      (else
        (`/Game/Core/Blueprint/Player/BP_BubbleCharacter.ReloadingFeedback` (`self.Owning Character`))))))

(fn `Base Fire`
  (set `self.ShootDelayTime` 0.5)
  (`|SpawnActorFromClass` "/Game/Core/Blueprint/BP_PRojectile.BP_PRojectile_C" (`self.Get Forward Projectile Spawn Transform`) "Undefined" "MultiplyWithRoot" null null)
  (set `self.CanShoot` false))

(fn `Get Forward Projectile Spawn Transform`
  (returns (ReturnValue :type "Transform Structure"))
  (bind _owning_character (`self.Owning Character`))
  (bind _returnvalue (`Actor.K2_GetActorRotation` _owning_character))
  (return (`KismetMathLibrary.MakeTransform` (+ (`SceneComponent.GetSocketLocation` (`Character.Mesh` _owning_character) "Head") (`KismetMathLibrary.GreaterGreater_VectorRotator` (`self.Bubble offset`) _returnvalue)) _returnvalue)))

(fn `Get Projectile Spawn Transform With Angle Offset`
  (params (`Angle Offset` :type "Float (double-precision)"))
  (returns (ReturnValue :type "Transform Structure"))
  (bind _owning_character (`self.Owning Character`))
  (bind (_returnvalue_roll _returnvalue_pitch _returnvalue_yaw) (`KismetMathLibrary.BreakRotator` (`Actor.K2_GetActorRotation` _owning_character)))
  (return (`KismetMathLibrary.MakeTransform` (+ (* (`KismetMathLibrary.GreaterGreater_VectorRotator` (`Actor.GetActorForwardVector` _owning_character) (`KismetMathLibrary.MakeRotator` 0.0 0.0 `Angle Offset`)) 100) (`Actor.K2_GetActorLocation` _owning_character)) (`KismetMathLibrary.MakeRotator` 0.0 0.0 (+ _returnvalue_yaw `Angle Offset`)))))

(fn `Rear Fire`
  (if (`self.RearFirePowerup`)
    (`|SpawnActorFromClass` "/Game/Core/Blueprint/BP_PRojectile.BP_PRojectile_C" (`self.Get Projectile Spawn Transform With Angle Offset` 180.0) "Undefined" "MultiplyWithRoot" null null)))

(fn `Shot Reset Timer`
  (params (DeltaTime :type "Float (double-precision)"))
  (if (not (`self.CanShoot`))
    (bind _output_get (set `self.ShootDelayTimer` (+ DeltaTime (`self.ShootDelayTimer`))))
    (if (>= _output_get (`self.ShootDelayTime`))
      (set `self.CanShoot` true)
      (set `self.ShootDelayTimer` 0.0))))

(fn `Spread Fire 1`
  (if (`self.SpreadFire1Powerup`)
    (`|SpawnActorFromClass` "/Game/Core/Blueprint/BP_PRojectile.BP_PRojectile_C" (`self.Get Projectile Spawn Transform With Angle Offset` 10.0) "Undefined" "MultiplyWithRoot" null null)
    (`|SpawnActorFromClass` "/Game/Core/Blueprint/BP_PRojectile.BP_PRojectile_C" (`self.Get Projectile Spawn Transform With Angle Offset` -10.0) "Undefined" "MultiplyWithRoot" null null)))

(fn `Spread Fire 2`
  (if (`self.SpreadFire2Powerup`)
    (`|SpawnActorFromClass` "/Game/Core/Blueprint/BP_PRojectile.BP_PRojectile_C" (`self.Get Projectile Spawn Transform With Angle Offset` 20.0) "Undefined" "MultiplyWithRoot" null null)
    (`|SpawnActorFromClass` "/Game/Core/Blueprint/BP_PRojectile.BP_PRojectile_C" (`self.Get Projectile Spawn Transform With Angle Offset` -20.0) "Undefined" "MultiplyWithRoot" null null)))