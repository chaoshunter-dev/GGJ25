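; Interactable laser-puzzle mirror that rotates in 45-degree steps and redirects a laser beam.
; Interaction hides the laser on every spinning mirror, then Tick turns the mesh until it snaps to the next yaw and tells the Emitter to update.
; ReflectLaser traces from the left or right arrow and stretches a child-actor cable to the hit as the beam.
; Hits chain recursively into tagged mirrors or activate a BP_LaserReceiver.
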(event `self.ReceiveBeginPlay`
  (bind _ascable_actor (cast `CableActor` (`ChildActorComponent.ChildActor` (`self.ChildCable`))))
  (bind _ascable_component (cast `CableComponent` (`Actor.RootComponent` _ascable_actor)))
  (set `self.CableComponent` _ascable_component))

(event `self.ReceiveTick`
  (params (DeltaSeconds :type "Float (single-precision)"))
  (`parent.ReceiveTick` DeltaSeconds)
  (if (`self.ShouldTowerTurn`)
    (`self.TurnMirror` DeltaSeconds)
    (bind _finished (`self.CheckReachedNextRotationGoal`))
    (if _finished
      (`self.ClampNextRotationBetween180`))))

(event `Event ReflectLaser`
  (params (ReflectLeft :type Boolean))
  (bind _cablecomponent (`self.CableComponent`))
  (bind _returnvalue (`SceneComponent.K2_GetComponentToWorld` (`self.CableComponent`)))
  (`SceneComponent.SetVisibility` (`self.CableComponent`) true false)
  (if ReflectLeft
    (`KismetSystemLibrary.PrintString` "Reflect Left")
    (`self.GetLeftTraceLocations`)
    (else
      (`self.GetRightTraceLocations`)))
  (bind _outhit (`KismetSystemLibrary.LineTraceSingle` (`self.Trace Start`) (`self.Trace End`) "TraceTypeQuery1"))
  (`|ExecutionSequence`
    (:`then_0`
      (bind (_bblockinghit _binitialoverlap _time _distance _location _impactpoint _normal _impactnormal _physmat _hitactor _hitcomponent) (`GameplayStatics.BreakHitResult` _outhit))
      (bind _asbp_spinning_mirror (cast `/Game/Core/Blueprint/Interactables/Mirror/BP_SpinningMirror` _hitactor))
      (bind _componenttags (`ActorComponent.ComponentTags` _hitcomponent))
      (if (== (`|GetArrayItem` _componenttags) "Mirror")
        (`self.Event ReflectLaser` _asbp_spinning_mirror (== (`|GetArrayItem` _componenttags 1) "Right"))))
    (:`then_1`
      (if (`KismetMathLibrary.EqualExactly_VectorVector` _impactpoint)
        (set `CableComponent.EndLocation` (`KismetMathLibrary.InverseTransformLocation` _returnvalue (`self.Trace End`)) _cablecomponent)
        (else
          (set `CableComponent.EndLocation` (`KismetMathLibrary.InverseTransformLocation` _returnvalue _impactpoint) _cablecomponent))))
    (:`then_2`
      (bind _asbp_laser_receiver (cast `/Game/Core/Blueprint/Puzzles/Mirror/BP_LaserReceiver` _hitactor))
      (`/Game/Core/Blueprint/Puzzles/Mirror/BP_LaserReceiver.Event Activate` _asbp_laser_receiver))))

(fn `CheckReachedNextRotationGoal`
  (returns (Finished :type Boolean))
  (bind _returnvalue (>= (`self.TurnTracker`) 45.0))
  (if _returnvalue
    (set `self.TurnTracker` 0.0)
    (set `self.ShouldTowerTurn` false)
    (`SceneComponent.K2_SetWorldRotation` (`self.SM_Mirror`) (`KismetMathLibrary.MakeRotator` 0.0 0.0 (`self.NextRotation`)) false false)
    (set `self.NextRotation` (+ (`self.NextRotation`) 45.0))
    (`/Game/Core/Blueprint/Puzzles/Mirror/BP_LaserEmitter.Event UpdateLaser` (`self.Emitter`))
    (return (not _returnvalue))))

(fn `ClampNextRotationBetween180`
  (if (> (`self.NextRotation`) 180.0)
    (set `self.NextRotation` -135.0)))

(fn `GetLeftTraceLocations`
  (bind _leftarrow (`self.LeftArrow`))
  (bind _returnvalue (`SceneComponent.K2_GetComponentLocation` _leftarrow))
  (set `self.Trace Start` _returnvalue)
  (set `self.Trace End` (+ _returnvalue (* (`SceneComponent.GetForwardVector` _leftarrow) 10000.0))))

(fn `GetRightTraceLocations`
  (bind _rightarrow (`self.RightArrow`))
  (bind _returnvalue (`SceneComponent.K2_GetComponentLocation` _rightarrow))
  (set `self.Trace Start` _returnvalue)
  (set `self.Trace End` (+ _returnvalue (* (`SceneComponent.GetForwardVector` _rightarrow) 10000.0))))

(fn `TriggerInteraction`
  (`parent.TriggerInteraction`)
  (set `self.ShouldTowerTurn` true)
  (bind _outactors (`GameplayStatics.GetAllActorsOfClass` "BP_SpinningMirror_C"))
  (for _array_element _outactors
    (`self.Turn Off Laser` _array_element)))

(fn `Turn Off Laser`
  (`SceneComponent.SetVisibility` (`self.CableComponent`) false false))

(fn `TurnMirror`
  (params (DeltaTime :type "Float (double-precision)"))
  (bind _returnvalue (* DeltaTime (`self.RotationSpeed`)))
  (`SceneComponent.K2_AddWorldRotation` (`self.SM_Mirror`) (`KismetMathLibrary.MakeRotator` 0.0 0.0 _returnvalue) false false)
  (set `self.TurnTracker` (+ (`self.TurnTracker`) _returnvalue)))

(fn `UserConstructionScript`
  (bind _startrotation (`self.StartRotation`))
  (`parent.UserConstructionScript`)
  (`SceneComponent.K2_SetRelativeRotation` (`self.SM_Mirror`) (`KismetMathLibrary.MakeRotator` 0.0 0.0 _startrotation) false false)
  (set `self.NextRotation` (+ _startrotation 45.0)))